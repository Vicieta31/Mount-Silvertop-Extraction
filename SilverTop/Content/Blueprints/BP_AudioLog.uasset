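; BP_AudioLog is an audio log trigger that plays its Sound in 2D when the first-person character begins overlapping its Box.
; Automatic logs trigger directly, while others require the character's AudioStart flag to be true at the moment of overlap.
; Both routes share one playback check that uses Played to limit it to one play, and nothing plays when PlayOnce is off.
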(event `self.Box.OnComponentBeginOverlap`
  (params (OverlappedComponent :type "PrimitiveComponent Object Reference") (OtherActor :type "Actor Object Reference") (OtherComp :type "PrimitiveComponent Object Reference") (OtherBodyIndex :type Integer) (bFromSweep :type Boolean) (SweepResult :type "HitResult Structure (by ref)"))
  (bind _asbp_first_person_character (cast `/Game/FirstPerson/Blueprints/BP_FirstPersonCharacter` OtherActor))
  (if (`self.automatic?`)
    (if (`self.playOnce?`) :!label _label
      (if (not (`self.played?`))
        (set `self.played?` true)
        (`GameplayStatics.PlaySound2D` (`self.Sound`) 1.0 1.0 0.0 null null)))
    (elif (`/Game/FirstPerson/Blueprints/BP_FirstPersonCharacter.audioStart` _asbp_first_person_character)
      (goto _label))))

(fn `UserConstructionScript`)