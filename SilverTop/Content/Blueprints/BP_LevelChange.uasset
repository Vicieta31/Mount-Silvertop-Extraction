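; BP_LevelChange is a trigger actor that moves the player to another level when its box is overlapped.
; On BeginPlay it caches the first-person player character.
; On overlap it fades the camera out, disables the character's movement, waits for the fade to finish, then opens the referenced level.
; The overlap does not check which actor entered the box.
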(event `self.ReceiveBeginPlay`
  (bind _asbp_first_person_character (cast `/Game/FirstPerson/Blueprints/BP_FirstPersonCharacter` (`GameplayStatics.GetPlayerCharacter` 0))))

(event `self.Box.OnComponentBeginOverlap`
  (params (OverlappedComponent :type "PrimitiveComponent Object Reference") (OtherActor :type "Actor Object Reference") (OtherComp :type "PrimitiveComponent Object Reference") (OtherBodyIndex :type Integer) (bFromSweep :type Boolean) (SweepResult :type "HitResult Structure (by ref)"))
  ;[1 1 1] Transicion a NextLevel
  (`PlayerCameraManager.StartCameraFade` (`GameplayStatics.GetPlayerCameraManager` 0) 0.0 1.0 1.6 (`self.Color`) false false)
  (`CharacterMovementComponent.DisableMovement` (`Character.CharacterMovement` (stale `self.ReceiveBeginPlay` _asbp_first_person_character)))
  (`KismetSystemLibrary.Delay` 1.6)
  (`GameplayStatics.OpenLevelBySoftObjectPtr` (`self.Level`)))

(fn `UserConstructionScript`)