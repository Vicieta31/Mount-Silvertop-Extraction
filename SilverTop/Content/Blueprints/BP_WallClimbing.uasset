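; BP_WallClimbing is a climbable-area trigger that tells BP_FirstPersonCharacter when it is within climbing range.
; On Box overlap it sets the character's Ladder flag, passes the Box's forward vector as OtherVectorRight and prints that vector.
; When overlap ends it clears the Ladder and Climbing flags and calls NotOnLadder on the character.
; The actor only supplies state and direction, with no climbing movement of its own.
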(event `self.Box.OnComponentBeginOverlap`
  (params (OverlappedComponent :type "PrimitiveComponent Object Reference") (OtherActor :type "Actor Object Reference") (OtherComp :type "PrimitiveComponent Object Reference") (OtherBodyIndex :type Integer) (bFromSweep :type Boolean) (SweepResult :type "HitResult Structure (by ref)"))
  (bind _asbp_first_person_character (cast `/Game/FirstPerson/Blueprints/BP_FirstPersonCharacter` OtherActor))
  (set `/Game/FirstPerson/Blueprints/BP_FirstPersonCharacter.ladder` true _asbp_first_person_character)
  (bind _output_get (set `/Game/FirstPerson/Blueprints/BP_FirstPersonCharacter.OtherVectorRight` (`SceneComponent.GetForwardVector` (`self.Box`)) _asbp_first_person_character))
  (`KismetSystemLibrary.PrintText` (`KismetTextLibrary.Conv_VectorToText` _output_get)))

(event `self.Box.OnComponentEndOverlap`
  (params (OverlappedComponent :type "PrimitiveComponent Object Reference") (OtherActor :type "Actor Object Reference") (OtherComp :type "PrimitiveComponent Object Reference") (OtherBodyIndex :type Integer))
  (bind _asbp_first_person_character (cast `/Game/FirstPerson/Blueprints/BP_FirstPersonCharacter` OtherActor))
  (set `/Game/FirstPerson/Blueprints/BP_FirstPersonCharacter.ladder` false _asbp_first_person_character)
  (set `/Game/FirstPerson/Blueprints/BP_FirstPersonCharacter.climbing` false _asbp_first_person_character)
  (`/Game/FirstPerson/Blueprints/BP_FirstPersonCharacter.notOnLadder` _asbp_first_person_character))

(fn `UserConstructionScript`)